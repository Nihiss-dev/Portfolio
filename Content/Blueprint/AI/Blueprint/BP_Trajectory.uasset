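; BP_Trajectory is an AI trajectory actor that visualizes a closed loop of points stored in MPoints.
; DrawDebug, run from the construction script and OnPointUpdated, adds a spline from each point to the next, wrapping last to first.
; It also adds an arrow and index label at each point, rotated toward the next.
; AddPoint delegates to AddTrajectoryPoint, and a separate debug-line helper is unused here.
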(fn `AddPoint`
  (`self.AddTrajectoryPoint`))

(fn `DrawDebug`
  (bind _m_points (`self.m_Points`))
  (for (_array_element _array_index) _m_points
    (`|ExecutionSequence`
      (:`then_0`
        (bind _returnvalue (`AddComponent|NODE_AddSplineComponent-1`))
        (bind _returnvalue_2 (`SceneComponent.K2_GetComponentLocation` _array_element))
        (bind _returnvalue_3 (`SceneComponent.K2_GetComponentLocation` (`|GetArrayItem` _m_points (`KismetMathLibrary.SelectInt` 0 (+ _array_index 1) (== _array_index (`KismetArrayLibrary.Array_LastIndex` _m_points))))))
        (`SplineComponent.SetSplinePoints` _returnvalue (`|MakeArray` _returnvalue_2 _returnvalue_3) "World" true))
      (:`then_1`
        (bind _returnvalue_location (`KismetMathLibrary.BreakTransform` (`KismetMathLibrary.MakeRelativeTransform` (`SceneComponent.K2_GetComponentToWorld` _array_element) (`self.GetTransform`))))
        (bind _returnvalue_4 (`KismetMathLibrary.FindLookAtRotation` _returnvalue_2 _returnvalue_3))
        (`AddComponent|NODE_AddArrowComponent-1` :`RelativeTransform` (`KismetMathLibrary.MakeTransform` _returnvalue_location _returnvalue_4))
        (bind _returnvalue_5 (`AddComponent|NODE_AddTextRenderComponent-1` :`RelativeTransform` (`KismetMathLibrary.MakeTransform` _returnvalue_location _returnvalue_4)))
        (`TextRenderComponent.K2_SetText` _returnvalue_5 (`KismetTextLibrary.Conv_IntToText` _array_index))))))

(fn `DrawLineBetweenPoints`
  (params (StartPoint :type "SceneComponent Object Reference") (EndPoint :type "SceneComponent Object Reference"))
  (`KismetSystemLibrary.DrawDebugLine` (`SceneComponent.K2_GetComponentLocation` StartPoint) (`SceneComponent.K2_GetComponentLocation` EndPoint) (struct :`R` 0.609375 :`G` 0.011874 :`A` 1.0) 90.0 5.0))

(fn `OnPointUpdated`
  (`self.DrawDebug`))

(fn `UserConstructionScript`
  (locals (CurrentIndex :type Integer))
  (`self.DrawDebug`))