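; AI controller for guard characters that patrols and detects the player through perception.
; On BeginPlay it runs the BT_Patrol behavior tree.
; Perception updates write any sensed first-person character to the Enemy blackboard key.
; Target updates set CanSeePlayer from whether the stimulus was successfully sensed, without checking which actor triggered it.
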(event `self.ReceiveBeginPlay`
  (`self.RunBehaviorTree` "/Game/Blueprint/AI/BehaviorTree/BT_Patrol.BT_Patrol"))

(event `self.AIPerception.OnPerceptionUpdated`
  (params (UpdatedActors :type "Array of Actor Object Reference (by ref)"))
  (for _array_element UpdatedActors
    (bind _asbp_first_person_character (cast `/Game/Blueprint/Player/FirstPerson/Blueprints/BP_FirstPersonCharacter` _array_element))
    (`BlackboardComponent.SetValueAsObject` (`self.Blackboard`) "Enemy" _asbp_first_person_character)))

(event `self.AIPerception.OnTargetPerceptionForgotten`
  (params (Actor :type "Actor Object Reference")))

(event `self.AIPerception.OnTargetPerceptionUpdated`
  (params (Actor :type "Actor Object Reference") (Stimulus :type "AIStimulus Structure"))
  (`BlackboardComponent.SetValueAsBool` (`self.Blackboard`) "CanSeePlayer" Stimulus_bSuccessfullySensed))

(fn `UserConstructionScript`)